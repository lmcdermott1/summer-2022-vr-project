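; BP_Saber is a grabbable VR lightsaber with a blade that extends and retracts on trigger press.
; Tick interpolates the blade's Z scale toward a target length set by the trigger toggle, with a sound for each direction.
; The first grab starts attached music and mutes the pawn's background sound.
; Dropping fades valid music, restores background volume after a delay, and retracts an extended blade.
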(event OnGrabbed(GrabComponent)
  (Utilities|FlowControl|DoOnce false
    (:Completed
      (bind _returnvalue (Audio|SpawnSoundAttached "/Game/Audio/Saber/StarWarsEdit.StarWarsEdit" (Variables|Default|GetHandle) "None" "0, 0, 0" "0, 0, 0" "KeepRelativeOffset" false 1.0 1.0 0.5 0 0))
      (Variables|Default|SetMusic _returnvalue)
      (Audio|Components|Audio|SetVolumeMultiplier (Variables|/Game/VRCharacterPawn.VRCharacterPawn_C|GetBackground%20Sound (Variables|Default|GetChar%20Ref)) 0.0 :!class /Script/Engine.AudioComponent))))

(event OnDropped(GrabComponent)
  (bind _music (Variables|Default|GetMusic))
  (Utilities|IsValid _music
    (:Is%20Valid
      (Audio|Components|Audio|AdjustVolume _music 2.0 0.0 "Linear" :!class /Script/Engine.AudioComponent)
      (Utilities|FlowControl|Delay 1.0)
      (Audio|Components|Audio|SetVolumeMultiplier (Variables|/Game/VRCharacterPawn.VRCharacterPawn_C|GetBackground%20Sound (Variables|Default|GetChar%20Ref)) 0.25 :!class /Script/Engine.AudioComponent))
    (:Is%20Not%20Valid
      _))
  (if (Variables|Default|GetBladeVisible)
    (Variables|Default|SetTargetBladeLength 0.0)
    (Variables|Default|SetBladeVisible false)
    (Audio|SpawnSoundAttached "/Game/Audio/Saber/fx5.fx5" (Variables|Default|GetSaberBlade) "None" "0, 0, 0" "0, 0, 0" "KeepRelativeOffset" false 0.7 1.0 0.0 0 0)))

(event EventBeginPlay
  (Rendering|SetVisibility (Variables|Default|GetSaberBlade) true true)
  (Variables|Default|SetBladeVisible false)
  (bind _asvrcharacter_pawn (Utilities|Casting|CastToVRCharacterPawn (Game|Player|GetPlayerPawn 0)))
  (Variables|Default|SetChar%20Ref _asvrcharacter_pawn))

(event Collision|EventActorBeginOverlap
  (params (OtherActor :type Actor%20Object%20Reference)))

(event EventTick
  (params (DeltaSeconds :type Float%20%28single-precision%29))
  (bind _saberblade (Variables|Default|GetSaberBlade))
  (bind _returnvalue (Transformation|GetWorldScale _saberblade))
  (Transformation|SetWorldScale3D _saberblade (Math|Vector|MakeVector (.x _returnvalue) (.y _returnvalue) (Math|Interpolation|FInterpTo (.z _returnvalue) (Variables|Default|GetTargetBladeLength) DeltaSeconds (Variables|Default|GetBladeSpeed)))))

(event EventTriggerPressed
  (bind _saberblade (Variables|Default|GetSaberBlade))
  (if (Variables|Default|GetBladeVisible)
    (Variables|Default|SetTargetBladeLength 0.0)
    (Variables|Default|SetBladeVisible false)
    (Audio|SpawnSoundAttached "/Game/Audio/Saber/fx5.fx5" _saberblade "None" "0, 0, 0" "0, 0, 0" "KeepRelativeOffset" false 0.7 1.0 0.5 0 0)
    (else
      (Variables|Default|SetTargetBladeLength (Variables|Default|GetMaxBladeLength))
      (Variables|Default|SetBladeVisible true)
      (Audio|SpawnSoundAttached "/Game/Audio/Saber/fx4_1.fx4_1" _saberblade "None" "0, 0, 0" "0, 0, 0" "KeepRelativeOffset" false 0.7 1.0 0.2 0 0))))

(fn ConstructionScript
  (Transformation|AttachComponentToComponent (Variables|Default|GetSaberBlade) (Variables|Default|GetHandle) "None" "KeepRelative" "KeepRelative" "KeepRelative" true))
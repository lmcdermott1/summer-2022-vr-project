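; A grabbable whiteboard marker that draws on a BP_WB_Working board in its configured color.
; BeginPlay applies the matching material to the marker meshes and, after a short delay, saves its home transform.
; While its box overlaps the board's ZirousDeskTabletop component, Tick line-traces along the arrow and passes the hit collision UV and color to DrawOnWB.
; When dropped, it snaps home after a delay unless held again.
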(event OnComponentBeginOverlap(Box)
  (params (OverlappedComponent :type Primitive%20Component%20Object%20Reference) (OtherActor :type Actor%20Object%20Reference) (OtherComp :type Primitive%20Component%20Object%20Reference) (OtherBodyIndex :type Integer) (bFromSweep :type Boolean) (SweepResult :type Hit%20Result%20Structure%20%28by%20ref%29))
  (bind _asbp_wb_working (Utilities|Casting|CastToBP_WB_Working OtherActor))
  (if (== (Variables|/Game/Tour/Whiteboard/SecondAttempt/BP_WB_Working.BP_WB_Working_C|GetZirous_Desk_Tabletop _asbp_wb_working) OtherComp)
    (Variables|Default|SetInUse true)))

(event OnComponentEndOverlap(Box)
  (params (OverlappedComponent :type Primitive%20Component%20Object%20Reference) (OtherActor :type Actor%20Object%20Reference) (OtherComp :type Primitive%20Component%20Object%20Reference) (OtherBodyIndex :type Integer))
  (Variables|Default|SetInUse false))

(event OnGrabbed(GrabComponent1)
  (Variables|Default|SetBeingHeld true))

(event OnDropped(GrabComponent1)
  (Variables|Default|SetBeingHeld false)
  (Utilities|FlowControl|Delay 4.0)
  (if (not (Variables|Default|GetBeingHeld))
    (Transformation|SetActorTransform (Variables|Default|GetSavedTransform))))

(event EventBeginPlay
  (bind _cone1 (Variables|Default|GetCone1))
  (switch Utilities|FlowControl|Switch|SwitchonEColor (Variables|Default|GetColor)
    (:NewEnumerator0
      (Rendering|Material|SetMaterial _cone1 0 "/Game/Tour/MaterialColors/Red.Red"))
    (:NewEnumerator3
      (Rendering|Material|SetMaterial _cone1 0 "/Game/Tour/MaterialColors/Green.Green"))
    (:NewEnumerator4
      (Rendering|Material|SetMaterial _cone1 0 "/Game/Tour/MaterialColors/Blue.Blue"))
    (:NewEnumerator8
      (Rendering|Material|SetMaterial (Variables|Default|GetCylinder1) 0 "/Game/Tour/MaterialColors/Black.Black")))
  (Utilities|FlowControl|Delay 0.3)
  (Variables|Default|SetSavedTransform (Transformation|GetActorTransform)))

(event EventTick
  (params (DeltaSeconds :type Float%20%28single-precision%29))
  (bind _arrow1 (Variables|Default|GetArrow1))
  (bind _returnvalue (Transformation|GetWorldLocation _arrow1))
  (if (Variables|Default|GetInUse)
    (bind (_outhit _returnvalue_2) (Collision|LineTraceByChannel _returnvalue (+ _returnvalue (* (Math|Vector|GetForwardVector _arrow1) 5e+02)) "TraceTypeQuery1" true 0 "None"))
    (if _returnvalue_2
      (bind _asbp_wb_working (Utilities|Casting|CastToBP_WB_Working (.HitActor (Collision|BreakHitResult _outhit))))
      (Default|DrawonWB _asbp_wb_working (.UV (Class|GameplayStatics|FindCollisionUV _outhit)) (Variables|Default|GetColor)))))

(fn ConstructionScript)
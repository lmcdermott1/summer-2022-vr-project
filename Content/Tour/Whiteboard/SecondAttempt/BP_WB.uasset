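; BP_WB is a paintable whiteboard actor that draws brush strokes onto its static mesh surface.
; On BeginPlay it creates a render target, binds it to the mesh's dynamic material as the BrushStroke texture, and creates a dynamic brush material.
; Its Trace event converts a hit into a UV position, sets brush color, size and strength, then draws the brush material into the render target.
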(event Custom|Trace
  (params (BrushColor :type Color%20Structure) (BrushSize :type Float%20%28single-precision%29) (BrushStrength :type Float%20%28single-precision%29) (Hit :type Hit%20Result%20Structure))
  (bind _uv (Class|GameplayStatics|FindCollisionUV Hit))
  (bind (_x _y) (Math|Vector2D|BreakVector2D _uv))
  ;[1 1 1] 9:55
  (Rendering|Material|SetVectorParameterValue (Variables|Default|GetBrush%20MI) "HitPosition" (Utilities|Struct|MakeLinearColor _x _y 0.0 1.0) :!class /Script/Engine.MaterialInstanceDynamic)
  (Rendering|Material|SetScalarParameterValue (Variables|Default|GetBrush%20MI) "BrushSize" BrushSize :!class /Script/Engine.MaterialInstanceDynamic)
  (Rendering|Material|SetVectorParameterValue (Variables|Default|GetBrush%20MI) "BrushColor" (Math|Conversions|ToLinearColor(Color) BrushColor) :!class /Script/Engine.MaterialInstanceDynamic)
  (Rendering|Material|SetScalarParameterValue (Variables|Default|GetBrush%20MI) "BrushStrength" BrushStrength :!class /Script/Engine.MaterialInstanceDynamic)
  (Rendering|DrawMaterialtoRenderTarget (Variables|Default|GetRender) (Variables|Default|GetBrush%20MI)))

(event EventBeginPlay
  (bind _returnvalue (Rendering|Material|CreateDynamicMaterialInstance (Variables|Default|GetStaticMesh) 0 "/Game/Tour/Whiteboard/SecondAttempt/MI_WB.MI_WB" "None" :!class /Script/Engine.PrimitiveComponent))
  ;[1 1 1] May need to adjust size
  (bind _returnvalue_2 (Rendering|CreateRenderTarget2D 512 512 "RTF_RGBA16f"))
  (Variables|Default|SetRender _returnvalue_2)
  (Rendering|Material|SetTextureParameterValue _returnvalue "BrushStroke" _returnvalue_2)
  (bind _returnvalue_3 (Rendering|Material|CreateDynamicMaterialInstance "/Game/Tour/Whiteboard/SecondAttempt/MI_Brush.MI_Brush" "None" "None" :!class /Script/Engine.KismetMaterialLibrary))
  (Variables|Default|SetBrush%20MI _returnvalue_3))

(event Collision|EventActorBeginOverlap
  (params (OtherActor :type Actor%20Object%20Reference)))

(event EventTick
  (params (DeltaSeconds :type Float%20%28single-precision%29)))

(fn ConstructionScript)
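; Drawable whiteboard actor that paints colored marks onto a render target and wipes it clean.
; BeginPlay clears the canvas and creates a dynamic whiteboard material on the tabletop mesh, plus a marker material this graph never uses.
; DrawOnWB sets color (red, green, blue or near-black) and UV location on the whiteboard material, then draws it into the render target.
; Any overlap with the ClearButton component clears the canvas.
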(event OnComponentBeginOverlap(ClearButton)
  (params (OverlappedComponent :type Primitive%20Component%20Object%20Reference) (OtherActor :type Actor%20Object%20Reference) (OtherComp :type Primitive%20Component%20Object%20Reference) (OtherBodyIndex :type Integer) (bFromSweep :type Boolean) (SweepResult :type Hit%20Result%20Structure%20%28by%20ref%29))
  (Rendering|ClearRenderTarget2D "/Game/Tour/WorkingWBOld/Canvas_RT.Canvas_RT"))

(event Custom|DrawOnWB
  (params (LocationToDraw :type Vector%202D%20Structure) (Color :type EColor%20Enum :default "NewEnumerator0"))
  (bind _wb (Variables|Default|GetWB))
  (bind _wb_2 (Variables|Default|GetWB))
  (switch Utilities|FlowControl|Switch|SwitchonEColor Color
    (:NewEnumerator0
      (Rendering|Material|SetVectorParameterValue _wb_2 "Color" "(R=1.000000,G=0.000000,B=0.000000,A=1.000000)" :!class /Script/Engine.MaterialInstanceDynamic))
    (:NewEnumerator3
      (Rendering|Material|SetVectorParameterValue _wb_2 "Color" "(R=0.000000,G=1.000000,B=0.000000,A=1.000000)" :!class /Script/Engine.MaterialInstanceDynamic))
    (:NewEnumerator4
      (Rendering|Material|SetVectorParameterValue _wb_2 "Color" "(R=0.000000,G=0.000000,B=1.000000,A=1.000000)" :!class /Script/Engine.MaterialInstanceDynamic))
    (:NewEnumerator8
      (Rendering|Material|SetVectorParameterValue _wb_2 "Color" "(R=0.001000,G=0.001000,B=0.001000,A=1.000000)" :!class /Script/Engine.MaterialInstanceDynamic)))
  (Rendering|Material|SetVectorParameterValue _wb "DrawLocation" (Math|Conversions|ToLinearColor(Vector) (Math|Conversions|ToVector(Vector2D) LocationToDraw)) :!class /Script/Engine.MaterialInstanceDynamic)
  (Rendering|DrawMaterialtoRenderTarget "/Game/Tour/WorkingWBOld/Canvas_RT.Canvas_RT" _wb))

(event EventBeginPlay
  (bind _returnvalue (Rendering|Material|CreateDynamicMaterialInstance (Variables|Default|GetZirous_Desk_Tabletop) 0 "/Game/Tour/WorkingWBOld/M_WhiteBoard.M_WhiteBoard" "None" :!class /Script/Engine.PrimitiveComponent))
  (Variables|Default|SetWB _returnvalue)
  (bind _returnvalue_2 (Rendering|Material|CreateDynamicMaterialInstance "/Game/Tour/WorkingWBOld/M_WBMarker.M_WBMarker" "None" "None" :!class /Script/Engine.KismetMaterialLibrary))
  (Variables|Default|SetMarker _returnvalue_2)
  (Rendering|ClearRenderTarget2D "/Game/Tour/WorkingWBOld/Canvas_RT.Canvas_RT"))

(fn ConstructionScript)
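; Tutorial audio actor that plays a wind sound whose volume rises as the VR character nears the actor.
; Tick maps distance from the VR root to a clamped volume multiplier, using a per-stage range from ClampingArray.
; MoveSoundComponent teleports the root to one of two hardcoded points by trigger number and advances the stage index.
; The sound spawns unattached, so these moves shift only the distance reference point.
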(event Custom|MoveSoundComponent
  (params (Trigger%20Number :type Integer))
  (bind _location (Variables|Default|GetLocation))
  (bind _defaultsceneroot (Variables|Default|GetDefaultSceneRoot))
  (switch int Trigger%20Number
    (:1
      (Transformation|SetWorldLocation _defaultsceneroot "-407.000000,-462.000000,29.000000" false true)
      (Math|Integer|IncrementInt _location))
    (:2
      (Transformation|SetWorldLocation _defaultsceneroot "295.000000,-735.000000,29.000000" false true)
      (Math|Integer|IncrementInt _location))))

(event EventBeginPlay
  (bind _clampingarray (Variables|Default|GetClampingArray))
  (Utilities|FlowControl|Sequence
    (:then_0
      (bind _returnvalue (Audio|SpawnSoundatLocation "/Game/MobileStarterContent/Audio/Starter_Wind06.Starter_Wind06" (Transformation|GetWorldLocation (Variables|Default|GetDefaultSceneRoot)) "0, 0, 0" 1.0 1.0 0.0 0 0))
      (Variables|Default|SetSound _returnvalue))
    (:then_1
      (Utilities|Array|Add _clampingarray (Math|Float|MakeLiteralFloat 6e+02))
      (Utilities|Array|Add _clampingarray (Math|Float|MakeLiteralFloat 9e+02))
      (Utilities|Array|Add _clampingarray (Math|Float|MakeLiteralFloat 8e+02)))))

(event Collision|EventActorBeginOverlap
  (params (OtherActor :type Actor%20Object%20Reference)))

(event EventTick
  (params (DeltaSeconds :type Float%20%28single-precision%29))
  (bind _sound (Variables|Default|GetSound))
  (if (Utilities|IsValid _sound)
    (Audio|Components|Audio|SetVolumeMultiplier _sound (Math|Float|MapRangeClamped (Math|Vector|Distance(Vector) (Transformation|GetWorldLocation (Variables|/Script/VRExpansionPlugin.VRCharacter|GetVRRootReference (Variables|Default|GetVR%20Character))) (Transformation|GetWorldLocation (Variables|Default|GetDefaultSceneRoot))) 0.0 (Utilities|Array|Get(acopy) (Variables|Default|GetClampingArray) (Variables|Default|GetLocation)) 12.0 2.0) :!class /Script/Engine.AudioComponent)
    (else
      (Development|PrintString "No"))))

(fn ConstructionScript)
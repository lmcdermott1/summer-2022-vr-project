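; SimpleAI4 is an AI pawn that follows the player's VRCharacterPawn and turns to face it.
; A loop started on BeginPlay re-issues AIMoveTo every 0.01 seconds, targeting the player at 300 units or farther and itself when closer, so it holds position.
; Each pass also smoothly interpolates the pawn's yaw toward the player with RInterpTo, without waiting for the move to finish.
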(event Custom|FollowPlayer
  (if (>= (Transformation|GetDistanceTo (Variables|Default|GetCharacter%20REF)) 3e+02)
    (AI|AIMoveTo self "0, 0, 0" (Variables|Default|GetCharacter%20REF) 5.0 false
      (:then
        (CallFunction|FacePlayer)))
    (else
      (AI|AIMoveTo self "0, 0, 0" self 5.0 false
        (:then
          (CallFunction|FacePlayer)))))
  (Utilities|FlowControl|Delay 0.01)
  (CallFunction|FollowPlayer))

(event Custom|Face%20Player
  (Transformation|SetActorRotation (Math|Rotator|MakeRotator 0.0 0.0 (.yaw (Math|Interpolation|RInterpTo (Transformation|GetActorRotation) (Math|Rotator|FindLookatRotation (Transformation|GetActorLocation) (Transformation|GetActorLocation (Variables|Default|GetCharacter%20REF))) (Utilities|Time|GetWorldDeltaSeconds) 7.5)))))

(event EventBeginPlay
  (bind _asvrcharacter_pawn (Utilities|Casting|CastToVRCharacterPawn (Game|GetPlayerCharacter 0)))
  (Variables|Default|SetCharacter%20REF _asvrcharacter_pawn)
  (CallFunction|FollowPlayer))

(fn ConstructionScript)